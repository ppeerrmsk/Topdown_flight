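; Base Blueprint for a player plane that flies along its forward vector at a throttle-controlled speed.
; The Thrust axis accumulates a clamped ThrustSpeed, which CurrentSpeed matches at once unless it is lower, in which case speed eases down using Drag as the interp rate.
; Tick moves the actor by world offset without sweep, so no collision check, then prints both speeds to screen for debugging.
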(event EventBeginPlay)

(event Collision|EventActorBeginOverlap
  (params (OtherActor :type Actor%20Object%20Reference)))

(event EventTick
  (params (DeltaSeconds :type Float%20%28single-precision%29))
  (bind _output_get (Variables|Default|SetDelta%20Seconds DeltaSeconds))
  (CallFunction|UpdatePosition _output_get)
  (CallFunction|PrintVariable))

(event Input|AxisEvents|InputAxisThrust
  (params (AxisValue :type Float%20%28single-precision%29))
  (Variables|Default|SetThrust%20Speed (Math|Float|Clamp(Float) (+ (* AxisValue (Utilities|Time|GetWorldDeltaSeconds) (Variables|Default|GetThrustMultiplier)) (Variables|Default|GetThrust%20Speed)) 0.0 (Variables|Default|GetMaxThrustSpeed))))

(fn ConstructionScript)

(fn UpdatePosition
  (params (Delta%20Seconds :type Float%20%28double-precision%29))
  ;[1 1 1] Speed(Current)
  (Variables|Default|SetCurrent%20Speed (select (< (Variables|Default|GetThrust%20Speed) (Variables|Default|GetCurrent%20Speed)) (Math|Interpolation|FInterpTo (Variables|Default|GetCurrent%20Speed) (Variables|Default|GetThrust%20Speed) Delta%20Seconds (Variables|Default|GetDrag)) (Variables|Default|GetThrust%20Speed)))
  ;[1 1 1] Position
  (bind _output_get (LocalVariables|SetNew%20Position (* (Transformation|GetActorForwardVector) (* (Variables|Default|GetCurrent%20Speed) (Variables|Default|GetDelta%20Seconds)))))
  (Transformation|AddActorWorldOffset _output_get))

(fn PrintVariable
  (Utilities|FlowControl|Sequence
    (:then_0
      (Development|PrintString (Utilities|String|Append "ThrustSpeed:" (Utilities|String|ToString(Float) (Variables|Default|GetThrust%20Speed))) true true "(R=0.000000,G=0.660000,B=1.000000,A=1.000000)" 1.0))
    (:then_1
      (Development|PrintString (Utilities|String|Append "Current Speed" (Utilities|String|ToString(Float) (Variables|Default|GetCurrent%20Speed))) true true "(R=0.000000,G=0.660000,B=1.000000,A=1.000000)" 1.0))))