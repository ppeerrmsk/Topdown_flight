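; Demo fighter aircraft actor for the 3D Radar system, carrying a RadarReturnBP component.
; The construction script copies the actor's faction tags into that component.
; When Flies is enabled, Tick moves it along its local forward axis and yaws it at a set turn rate, producing a simple circling flight.
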(event EventTick
  (params (DeltaSeconds :type Float%20%28single-precision%29))
  ;[1 1 1] Makes the aircraft fly around.
  (if (Variables|Default|GetFlies)
    (Transformation|AddActorLocalOffset (Math|Vector|MakeVector (* DeltaSeconds (Variables|Default|GetForward%20Speed)) 0.0 0.0) false false)
    (Transformation|AddActorLocalRotation (Math|Rotator|MakeRotator 0.0 0.0 (* DeltaSeconds (Variables|Default|GetTurn%20Rate))) false false)))

(fn ConstructionScript
  (Variables|/Game/3D_Radar/Blueprints/Radar_Return_BP.Radar_Return_BP_C|SetFaction%20Tags (Variables|Default|GetRadar_Return_BP) (Variables|Default|GetFactions%20Tags)))